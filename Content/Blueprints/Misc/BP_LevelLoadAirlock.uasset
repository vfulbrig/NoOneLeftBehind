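; Airlock actor that works two doors around sublevel loading, closing as loading begins and opening when it finishes.
; Begin and finish loading dispatchers drive Trigger or Untrigger on one door, chosen by whether the next sublevel is involved.
; Construction casts both child actors to BP_MovingPlatform, applying a door mesh and NoWitchBounce physical material.
; The stored references are crossed: ExitDoorActor comes from EntranceDoor, EntranceDoorActor from ExitDoor.
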(event Custom|Close%20Airlock
  (params (Next%20Sublevel%20Loading? :type Boolean))
  (if Next%20Sublevel%20Loading?
    (Default|Trigger (Variables|Internal|GetExit%20Door%20Actor))
    (else
      (Default|Untrigger (Variables|Internal|GetEntrance%20Door%20Actor)))))

(event Custom|Open%20Airlock
  (params (Next%20Sublevel%20Loaded? :type Boolean))
  (if Next%20Sublevel%20Loaded?
    (Default|Trigger (Variables|Internal|GetEntrance%20Door%20Actor))
    (else
      (Default|Untrigger (Variables|Internal|GetExit%20Door%20Actor)))))

(event EventBeginPlay
  (|CallParentFunction)
  (EventDispatchers|AssignDispatcheronBeginLoading (delegate Custom|Close%20Airlock))
  (EventDispatchers|AssignDispatcheronFinishLoading (delegate Custom|Open%20Airlock)))

(fn ConstructionScript
  (|CallParentFunction)
  (bind _door_actor (CallFunction|InitializeDoor (Variables|Default|GetEntrance%20Door)))
  (Variables|Internal|SetExit%20Door%20Actor _door_actor)
  (bind _door_actor_2 (CallFunction|InitializeDoor (Variables|Default|GetExit%20Door)))
  (Variables|Internal|SetEntrance%20Door%20Actor _door_actor_2))

(fn InitializeDoor
  (params (Door%20Child%20Component :type Child%20Actor%20Component%20Object%20Reference))
  (bind _asbp_moving_platform (Utilities|Casting|CastToBP_MovingPlatform (Variables|/Script/Engine.ChildActorComponent|GetChildActor Door%20Child%20Component)))
  (bind _output_get (LocalVariables|SetCasted%20Door _asbp_moving_platform))
  (Components|StaticMesh|SetStaticMesh (Variables|/Game/Blueprints/TriggeredObjects/BP_MovingPlatform.BP_MovingPlatform_C|GetMesh _output_get) (Variables|Parameters|GetDoor%20Static%20Mesh))
  (Class|PrimitiveComponent|SetPhysMaterialOverride (Variables|/Game/Blueprints/TriggeredObjects/BP_MovingPlatform.BP_MovingPlatform_C|GetMesh (LocalVariables|GetCasted%20Door)) "/Game/Blueprints/Misc/NoWitchBounce.NoWitchBounce")
  (return (LocalVariables|GetCasted%20Door)))