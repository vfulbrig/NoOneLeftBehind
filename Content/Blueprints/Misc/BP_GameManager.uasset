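; BP_GameManager tracks the characters in play and lets player controller 0 switch control between them.
; Functions add, remove and count entries in the CharactersInPlay array.
; The SwapCharacter event steps CurrentCharacterIndex backward or forward based on its Prev flag, wraps it at either end of the array, then possesses that character.
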(event EventBeginPlay)

(event Collision|EventActorBeginOverlap
  (params (OtherActor :type Actor%20Object%20Reference)))

(event EventTick
  (params (DeltaSeconds :type Float%20%28single-precision%29)))

(event Custom|Swap%20Character
  (params (Prev? :type Boolean))
  (Utilities|FlowControl|Sequence
    (:then_0
      ;[1 1 1] Set the current index to that of the character to be swapped to.
      (if Prev?
        (bind _result (Math|Integer|DecrementInt (Variables|CharacterSwapping|GetCurrent%20Character%20Index))
          (:%20%20
            (if (< _result 0)
              (Variables|CharacterSwapping|SetCurrent%20Character%20Index (Utilities|Array|LastIndex (Variables|CharacterSwapping|GetCharacters%20In%20Play))))))
        (else
          (bind _result_2 (Math|Integer|IncrementInt (Variables|CharacterSwapping|GetCurrent%20Character%20Index))
            (:%20%20
              (if (> _result_2 (Utilities|Array|LastIndex (Variables|CharacterSwapping|GetCharacters%20In%20Play)))
                (Variables|CharacterSwapping|SetCurrent%20Character%20Index 0)))))))
    (:then_1
      ;[1 1 1] Swap to the character
      (Pawn|Possess (Game|GetPlayerController 0) (Utilities|Array|Get(acopy) (Variables|CharacterSwapping|GetCharacters%20In%20Play) (Variables|CharacterSwapping|GetCurrent%20Character%20Index))))))

(fn ConstructionScript)

(fn AddCharacter
  (params (Character :type BP%20Character%20Base%20Object%20Reference))
  (Utilities|Array|Add (Variables|CharacterSwapping|GetCharacters%20In%20Play) Character))

(fn RemoveCharacter
  (params (Character :type BP%20Character%20Base%20Object%20Reference))
  (Utilities|Array|RemoveItem (Variables|CharacterSwapping|GetCharacters%20In%20Play) Character))

(fn GetNumCharactersinPlay
  (return (Utilities|Array|Length (Variables|CharacterSwapping|GetCharacters%20In%20Play))))