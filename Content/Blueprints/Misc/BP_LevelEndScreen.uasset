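; BP_LevelEndScreen is an actor that hosts the level end screen through a widget component showing WBP_ExitScreen.
; On BeginPlay it casts the component's widget, stores it, and copies the sector number and secrets values into it.
; If an alternate sector message is set, it passes that to the widget to override the displayed message.
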(event EventBeginPlay
  (bind _aswbp_exit_screen (Utilities|Casting|CastToWBP_ExitScreen (UserInterface|GetWidget (Variables|Default|GetEndScreenWidget))))
  (bind _output_get (Variables|Default|SetScreen%20Widget _aswbp_exit_screen))
  (Variables|/Game/Blueprints/UI/WBP_ExitScreen.WBP_ExitScreen_C|SetSector%20Number _output_get (Variables|Default|GetSector%20Number))
  (Variables|/Game/Blueprints/UI/WBP_ExitScreen.WBP_ExitScreen_C|SetSector%20Secrets _output_get (Variables|Default|GetSector%20Secrets))
  (if (not (Utilities|Text|TextIsEmpty (Variables|Default|GetAlt%20Sector%20Message)))
    (Default|SetSectorMessage (Variables|Default|GetScreen%20Widget) (Variables|Default|GetAlt%20Sector%20Message))))

(event Collision|EventActorBeginOverlap
  (params (OtherActor :type Actor%20Object%20Reference)))

(event EventTick
  (params (DeltaSeconds :type Float%20%28single-precision%29)))

(fn ConstructionScript)