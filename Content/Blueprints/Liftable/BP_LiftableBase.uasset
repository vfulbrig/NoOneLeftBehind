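; BP_LiftableBase is a base Blueprint for objects that can be lifted or grabbed.
; On BeginPlay it hands its Mesh to BPMarkObjectsComponent as the mesh to mark.
; One function toggles the mesh's physics simulation and collision together, switching between query-and-physics and no collision.
; Another reports whether it is inside another actor while grabbed, based on a nonzero ActorsOverlapping count.
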(event EventBeginPlay
  (Variables|/Game/MarkObjectSystem/Component/BP_MarkObjectsComponent.BP_MarkObjectsComponent_C|SetMeshes%20To%20Mark (Variables|Default|GetBP_MarkObjectsComponent) (Utilities|Array|MakeArray (Variables|Default|GetMesh))))

(fn ConstructionScript)

(fn SetLiftablePhysicsActive
  (params (Active? :type Boolean))
  (Physics|SetSimulatePhysics (Variables|Default|GetMesh) Active?)
  (Collision|SetCollisionEnabled (Variables|Default|GetMesh) (select Active? "QueryAndPhysics" "NoCollision")))

(fn InsideActorWhileGrabbed
  (return (> (Variables|Default|GetActors%20Overlapping) 0)))