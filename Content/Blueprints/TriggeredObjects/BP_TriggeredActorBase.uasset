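; Base Blueprint for triggered actors, providing shared Trigger and Untrigger functions that child classes override.
; Both default implementations only print a reminder that an override is needed.
; Initialize Switch Mesh tints a mesh material slot through a dynamic material instance, setting its Color parameter from the TriggerColor switch color or an optional override color.
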(event EventBeginPlay)

(event Collision|EventActorBeginOverlap
  (params (OtherActor :type Actor%20Object%20Reference)))

(event EventTick
  (params (DeltaSeconds :type Float%20%28single-precision%29)))

(fn ConstructionScript)

(fn Trigger
  (Development|PrintString "You need to override the Trigger function, silly!"))

(fn Untrigger
  (Development|PrintString "You need to override the Untrigger function, silly!"))

(fn InitializeSwitchMesh
  (params (Mesh :type Mesh%20Component%20Object%20Reference) (Material%20Index :type Integer))
  (bind _returnvalue (Rendering|Material|CreateDynamicMaterialInstance (Rendering|Material|GetMaterial Mesh Material%20Index) "None" "None" :!class /Script/Engine.KismetMaterialLibrary))
  (Rendering|Material|SetVectorParameterValue _returnvalue "Color" (Math|Color|SelectColor (Variables|Parameters|GetOverride%20Color) (CallFunction|SwitchColortoColor (Variables|Parameters|GetTrigger%20Color)) (Variables|Parameters|GetUse%20Override%20Color)) :!class /Script/Engine.MaterialInstanceDynamic)
  (Rendering|Material|SetMaterial Mesh Material%20Index _returnvalue))