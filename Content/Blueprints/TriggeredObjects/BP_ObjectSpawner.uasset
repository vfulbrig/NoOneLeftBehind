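; BP_ObjectSpawner is a triggerable actor that spawns one instance of a chosen class at its spawn point.
; Trigger replaces any existing spawned object with a fresh one, and Untrigger destroys it.
; The construction script shows the spawner's name and class to spawn as text tinted by its trigger color.
; When removed from the world, it can optionally destroy the object in play.
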(event EventBeginPlay)

(event Collision|EventActorBeginOverlap
  (params (OtherActor :type Actor%20Object%20Reference)))

(event EventTick
  (params (DeltaSeconds :type Float%20%28single-precision%29)))

(event EventEndPlay
  (params (EndPlayReason :type EEndPlayReason%20Enum :default "Destroyed"))
  (if (Math|Boolean|ANDBoolean (Utilities|Enum|Equal(Enum) EndPlayReason "RemovedFromWorld") (Variables|LoadSettings|GetRemove%20Object%20When%20Unloaded) (Utilities|IsValid (Variables|Internal|GetObject%20In%20Play)))
    (Actor|DestroyActor (Variables|Internal|GetObject%20In%20Play))))

(fn ConstructionScript
  (bind _trigger_color (Variables|Default|GetTrigger%20Color))
  (bind _color (CallFunction|SwitchColortoColor _trigger_color))
  (bind _returnvalue (Math|Conversions|ToColor(LinearColor) _color))
  ;[1 1 1] Display this actor's display name (since many spawners may be Colorless)
  (Rendering|Components|TextRender|SetText (Variables|Default|GetSpawner%20Title) (Utilities|Text|ToText(String) (Utilities|String|Append (Utilities|GetDisplayName self) (Utilities|String|MakeLiteralString " will spawn:"))))
  ;[1 1 1] Display the name of the actor class to be spawned.
  (Rendering|Components|TextRender|SetText (Variables|Default|GetObject%20Spawned%20Text) (select (Utilities|IsValidClass (Variables|Parameters|GetTo%20Spawn)) (Utilities|Text|ToText(String) (Utilities|GetClassDisplayName (Variables|Parameters|GetTo%20Spawn))) (Utilities|Text|MakeLiteralText "NOTHING!!!")))
  ;[1 1 1] Set the color of the text to be the spawner's Trigger Color.
  (Rendering|Components|TextRender|SetTextRenderColor (Variables|Default|GetSpawner%20Title) _returnvalue)
  (Rendering|Components|TextRender|SetTextRenderColor (Variables|Default|GetObject%20Spawned%20Text) _returnvalue))

(fn Trigger
  (Utilities|IsValid (Variables|Internal|GetObject%20In%20Play)
    (:Is%20Valid
      (CallFunction|DestroySpawnedObject))
    (:Is%20Not%20Valid
      _))
  (bind _returnvalue (Game|SpawnActorfromClass (Variables|Parameters|GetTo%20Spawn) (Transformation|GetWorldTransform (Variables|Transformation|GetObject%20Spawn%20Point)) "Undefined" 0 0))
  (Variables|Internal|SetObject%20In%20Play _returnvalue))

(fn DestroySpawnedObject
  (Actor|DestroyActor (Variables|Internal|GetObject%20In%20Play)))

(fn Untrigger
  (Utilities|IsValid (Variables|Internal|GetObject%20In%20Play)
    (:Is%20Valid
      (CallFunction|DestroySpawnedObject))))