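; BP_Door is a door in the triggered-objects set whose color reflects its trigger color.
; The construction script calls InitializeSwitchMesh, which creates a dynamic instance of Door_Color and applies it to the mesh's second material slot.
; Its Color parameter comes from the trigger's switch color, or from an override color when that option is enabled.
; The event graph is empty, so this graph contains no opening or movement logic.
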(event EventBeginPlay
  (|CallParentFunction) ; This node is disabled and will not be called.\nDrag off pins to build functionality.
)

(event Collision|EventActorBeginOverlap
  (params (OtherActor :type Actor%20Object%20Reference))
  (|CallParentFunction OtherActor) ; This node is disabled and will not be called.\nDrag off pins to build functionality.
)

(event EventTick
  (params (DeltaSeconds :type Float%20%28single-precision%29))
  (|CallParentFunction DeltaSeconds) ; This node is disabled and will not be called.\nDrag off pins to build functionality.
)

(fn ConstructionScript
  (CallFunction|InitializeSwitchMesh (Variables|Character|GetMesh) 1))

(fn InitializeSwitchMesh
  (params (Mesh :type Mesh%20Component%20Object%20Reference) (Material%20Index :type Integer))
  (bind _returnvalue (Rendering|Material|CreateDynamicMaterialInstance "/Game/Graphics/Materials/Door_Color.Door_Color" "None" "None" :!class /Script/Engine.KismetMaterialLibrary))
  (Rendering|Material|SetVectorParameterValue _returnvalue "Color" (Math|Color|SelectColor (Variables|Default|GetOverride%20Color) (CallFunction|SwitchColortoColor (Variables|Default|GetTrigger%20Color)) (Variables|Default|GetUse%20Override%20Color)) :!class /Script/Engine.MaterialInstanceDynamic)
  (Rendering|Material|SetMaterial Mesh Material%20Index _returnvalue))