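; BP_AntiMagicBarrier is a triggered barrier whose wall and collision switch on or off.
; Trigger and Untrigger toggle Collider collision and Wall visibility, with StartBarrierDisabled inverting both.
; A disabled start hides the wall at construction and drops collision on BeginPlay.
; The construction script builds top and bottom frames from mesh pieces, counted and spaced by actor scale, each passed to InitializeSwitchMesh.
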(event EventBeginPlay
  (|CallParentFunction)
  (if (Variables|Parameters|GetStart%20Barrier%20Disabled)
    (Collision|SetCollisionEnabled (Variables|Default|GetCollider) "NoCollision")))

(event Collision|EventActorBeginOverlap
  (params (OtherActor :type Actor%20Object%20Reference))
  (|CallParentFunction OtherActor) ; This node is disabled and will not be called.\nDrag off pins to build functionality.
)

(event EventTick
  (params (DeltaSeconds :type Float%20%28single-precision%29))
  (|CallParentFunction DeltaSeconds) ; This node is disabled and will not be called.\nDrag off pins to build functionality.
)

(fn ConstructionScript
  (|CallParentFunction)
  (Utilities|FlowControl|Sequence
    (:then_0
      ;[1 1 1] Make the top/bottom frame.
      (for _index (range 0 (- (Math|Float|Floor (.x (Transformation|GetActorScale3D))) 1))
        (CallFunction|SpawnFramePiece (* _index (/ 1e+02 (.x (Transformation|GetActorScale3D)))) 0.0)
        (CallFunction|SpawnFramePiece (* _index (/ 1e+02 (.x (Transformation|GetActorScale3D)))) (- 1e+02 (/ 2e+01 (.z (Transformation|GetActorScale3D)))))))
    (:then_1
      ;[1 1 1] Hide barrier if it is set to start disabled. The collision is disable on Begin Play.
      (if (Variables|Parameters|GetStart%20Barrier%20Disabled)
        (Rendering|SetVisibility (Variables|Default|GetWall) false false)))))

(fn SpawnFramePiece
  (params (Relative%20X :type Float%20%28double-precision%29) (Relative%20Z :type Float%20%28double-precision%29))
  (bind _returnvalue (AddComponent|AddStaticMeshComponent false (Math|Transform|MakeTransform (Math|Vector|MakeVector Relative%20X 0.0 Relative%20Z) "0, 0, 0" "1.000000,1.000000,1.000000")))
  (Components|StaticMesh|SetStaticMesh _returnvalue (Variables|Default|GetFrame%20Mesh))
  (Transformation|SetWorldScale3D _returnvalue "1.000000,1.000000,0.200000")
  (Rendering|Material|SetMaterial _returnvalue 0 "/Game/Graphics/Materials/M_ColoredWalls.M_ColoredWalls")
  (CallFunction|InitializeSwitchMesh _returnvalue))

(fn Trigger
  (Collision|SetCollisionEnabled (Variables|Default|GetCollider) (select (Variables|Parameters|GetStart%20Barrier%20Disabled) "QueryAndPhysics" "NoCollision"))
  (Rendering|SetVisibility (Variables|Default|GetWall) (Variables|Parameters|GetStart%20Barrier%20Disabled) false))

(fn Untrigger
  (Collision|SetCollisionEnabled (Variables|Default|GetCollider) (select (Variables|Parameters|GetStart%20Barrier%20Disabled) "NoCollision" "QueryAndPhysics"))
  (Rendering|SetVisibility (Variables|Default|GetWall) (not (Variables|Parameters|GetStart%20Barrier%20Disabled)) false))