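; BP_PressurePlateToggled is a pressure plate switch that flips between on and off each time it is pressed.
; Each press inverts the WasTrigged flag, calls TriggerSwitch or UntriggerSwitch accordingly, and lights or dims the button symbol to match.
; ForceWasTriggered sets the lit, triggered state directly without calling TriggerSwitch.
; A Debug flag prints a message on each toggle.
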(event EventBeginPlay
  (|CallParentFunction) ; This node is disabled and will not be called.\nDrag off pins to build functionality.
)

(fn ConstructionScript
  (|CallParentFunction))

(fn PressPressurePlate
  (CallFunction|SetButtonSymbolLit (not (Variables|Default|GetWasTrigged?)))
  (if (Variables|Default|GetWasTrigged?)
    (CallFunction|UntriggerSwitch)
    (else
      (CallFunction|TriggerSwitch)))
  (Variables|Default|SetWasTrigged? (not (Variables|Default|GetWasTrigged?)))
  (if (Variables|Default|GetDebug?)
    (if (Variables|Default|GetWasTrigged?)
      (Development|PrintString "Hello")
      (else
        (Development|PrintString "Goodbye")))))

(fn ForceWasTriggered
  (bind _output_get (Variables|Default|SetWasTrigged? true))
  (CallFunction|SetButtonSymbolLit _output_get))