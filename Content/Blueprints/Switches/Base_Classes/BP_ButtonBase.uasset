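; Base class for pressable button switches, built from a Button and Pedestal mesh.
; Construction initializes the Button as the switch mesh, and BeginPlay registers both meshes with the mark-objects component for marking.
; PressButton is a placeholder that prints a warning, leaving the actual press behavior to child classes.
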(event EventBeginPlay
  (|CallParentFunction)
  (Variables|/Game/MarkObjectSystem/Component/BP_MarkObjectsComponent.BP_MarkObjectsComponent_C|SetMeshes%20To%20Mark (Variables|Default|GetBP_MarkObjectsComponent) (Utilities|Array|MakeArray (Variables|Default|GetButton) (Variables|Default|GetPedestal))))

(fn ConstructionScript
  (CallFunction|InitializeSwitchMesh (Variables|Default|GetButton)))

(fn PressButton
  (Development|PrintString "You're using the base class silly!"))