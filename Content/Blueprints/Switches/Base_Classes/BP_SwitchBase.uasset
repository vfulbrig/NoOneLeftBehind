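; BP_SwitchBase is a base class for color-coded switches that trigger and untrigger linked actors.
; On BeginPlay it links manually assigned actors, plus any BP_TriggeredActorBase of matching TriggerColor unless the color is the exempt colorless value.
; TriggerSwitch and UntriggerSwitch relay calls to every linked actor.
; InitializeSwitchMesh tints a given mesh through a dynamic material instance to show the switch color.
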(event EventBeginPlay
  ;[1 1 1] Get the actors that will be affected by this switch
  (Utilities|Array|AppendArray (Variables|Internal|GetLinked%20Actors) (Variables|Parameters|GetOther%20Actors%20to%20Trigger))
  ;;[1 1 1] Get Triggerable Actors of the same color (unless this switch is colorless)
  (if (Utilities|Enum|NotEqual(Enum) (Variables|Parameters|GetTrigger%20Color) "NewEnumerator8")
    (bind _outactors (Actor|GetAllActorsOfClass "/Game/Blueprints/TriggeredObjects/BP_TriggeredActorBase.BP_TriggeredActorBase_C"))
    (for _array_element _outactors
      (if (Utilities|Enum|Equal(Enum) (Variables|Parameters|GetTrigger%20Color) (Variables|/Game/Blueprints/TriggeredObjects/BP_TriggeredActorBase.BP_TriggeredActorBase_C|GetTrigger%20Color _array_element))
        (Utilities|Array|AddUnique (Variables|Internal|GetLinked%20Actors) _array_element)))))

(event EventEndPlay
  (params (EndPlayReason :type EEndPlayReason%20Enum :default "Destroyed"))
  (if (Utilities|Enum|Equal(Enum) EndPlayReason "LevelTransition")
    (Utilities|Array|Clear (Variables|Internal|GetLinked%20Actors))))

(fn ConstructionScript)

(fn TriggerSwitch
  (for _array_element (Variables|Internal|GetLinked%20Actors)
    (Default|Trigger _array_element)))

(fn UntriggerSwitch
  (for _array_element (Variables|Internal|GetLinked%20Actors)
    (Default|Untrigger _array_element)))

(fn InitializeSwitchMesh
  (params (Mesh :type Mesh%20Component%20Object%20Reference))
  (bind _returnvalue (Rendering|Material|CreateDynamicMaterialInstance (Rendering|Material|GetMaterial Mesh (Variables|Default|GetColor%20Material%20Index)) "None" "None" :!class /Script/Engine.KismetMaterialLibrary))
  (Rendering|Material|SetVectorParameterValue _returnvalue "Color" (CallFunction|SwitchColortoColor (Variables|Parameters|GetTrigger%20Color)) :!class /Script/Engine.MaterialInstanceDynamic)
  (Rendering|Material|SetMaterial Mesh (Variables|Default|GetColor%20Material%20Index) _returnvalue))