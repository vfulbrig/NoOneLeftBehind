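; Base pressure plate switch that counts overlapping actors, pressing on the first to enter and releasing when the last leaves.
; Empty PressPressurePlate and UnpressPressurePlate functions act as hooks for child classes, called alongside forward or reverse timeline playback.
; The construction script caches raised and depressed mesh positions for the timeline lerp and creates a dynamic material for the glowing symbol.
; SetButtonSymbolLit switches that symbol between blue and black.
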(event EventBeginPlay
  (|CallParentFunction))

(event Collision|EventActorBeginOverlap
  (params (OtherActor :type Actor%20Object%20Reference))
  (Math|Integer|IncrementInt (Variables|Default|GetActors%20Pressing)
    (:%20%20
      ;[1 1 1] If the button was not already being pressed, trigger it.
      (if (== (Variables|Default|GetActors%20Pressing) 1)
        (Audio|Components|Audio|Play (Variables|Default|GetTL_PressurePlateAnim))
        (CallFunction|PressPressurePlate)
        (if (Variables|Default|GetDebug?)
          (Development|PrintString "Pressed!"))))))

(event EventEndPlay
  (params (EndPlayReason :type EEndPlayReason%20Enum :default "Destroyed"))
  (if (Utilities|Enum|Equal(Enum) EndPlayReason "RemovedFromWorld")
    _))

(event Collision|EventActorEndOverlap
  (params (OtherActor :type Actor%20Object%20Reference))
  (Math|Integer|DecrementInt (Variables|Default|GetActors%20Pressing)
    (:%20%20
      ;[1 1 1] Untrigger the button when the last object is removed from it.
      (if (== (Variables|Default|GetActors%20Pressing) 0)
        (CallFunction|UnpressPressurePlate)
        (Utilities|String|Reverse (Variables|Default|GetTL_PressurePlateAnim))
        (if (Variables|Default|GetDebug?)
          (Development|PrintString "Unpressed!"))))))

(fn ConstructionScript
  (bind _mesh (Variables|Default|GetMesh))
  (CallFunction|InitializeSwitchMesh (Variables|Default|GetMesh))
  ;[1 1 1] Create the glowing symbol's dynamic material.
  (bind _returnvalue (Rendering|Material|CreateDynamicMaterialInstance _mesh 1 (Rendering|Material|GetMaterial _mesh 1) "None" :!class /Script/Engine.PrimitiveComponent))
  (Variables|Internal|SetButton%20Symbol%20Material _returnvalue)
  ;[1 1 1] Button anim initialization
  (bind _output_get (Variables|Internal|SetButton%20Unpressed%20Point (Variables|/Script/Engine.SceneComponent|GetRelativeLocation (Variables|Default|GetMesh))))
  (Variables|Internal|SetButton%20Pressed%20Point (Math|Vector|MakeVector (.x _output_get) (.y _output_get) (- (.z _output_get) (Variables|Internal|GetDepress%20Distance)))))

(fn PressPressurePlate)

(fn UnpressPressurePlate)

(fn SetButtonSymbolLit
  (params (Button%20Symbol%20Lit? :type Boolean))
  (Rendering|Material|SetVectorParameterValue (Variables|Internal|GetButton%20Symbol%20Material) "Color" (Math|Color|SelectColor :A "(R=0.000000,G=0.000000,B=1.000000,A=1.000000)" :bPickA Button%20Symbol%20Lit?) :!class /Script/Engine.MaterialInstanceDynamic))