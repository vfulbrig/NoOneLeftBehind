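; BP_CharacterStrongman is a character Blueprint that defines how the Strongman throws a held actor.
; Charged Throw maps the throw charge, clamped between the drop threshold and maximum charge, to a force between drop and maximum throw force, with a slight upward force.
; Throw Pressed throws at drop force with a higher upward force.
; The event graph holds only disabled placeholder events, and construction defers to the parent.
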(event EventBeginPlay
  (|CallParentFunction) ; This node is disabled and will not be called.\nDrag off pins to build functionality.
)

(event Collision|EventActorBeginOverlap
  (params (OtherActor :type Actor%20Object%20Reference)))

(event EventTick
  (params (DeltaSeconds :type Float%20%28single-precision%29))
  (|CallParentFunction DeltaSeconds) ; This node is disabled and will not be called.\nDrag off pins to build functionality.
)

(fn ConstructionScript
  (|CallParentFunction))

(fn ChargedThrow
  (CallFunction|ThrowHeldActor (Math|Float|MapRangeClamped (Variables|Default|GetThrow%20Charge) (Variables|Default|GetDrop%20Charge%20Threshold) (Variables|Default|GetMax%20Throw%20Charge) (Variables|Default|GetDrop%20Force) (Variables|Default|GetMax%20Throw%20Force)) 1e+02))

(fn ThrowPressed
  (CallFunction|ThrowHeldActor (Variables|Default|GetDrop%20Force) 2e+02))