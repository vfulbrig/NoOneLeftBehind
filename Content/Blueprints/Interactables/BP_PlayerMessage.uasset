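; BP_PlayerMessage is an interactable object that shows dialogue text to the character who interacts with it.
; OnInteracted passes InteractMessages to that character as multi-page dialogue when it holds several entries, otherwise it displays the first entry as a single dialogue.
; The construction script adds the static mesh to the BPMarkObjectsComponent's list of meshes to mark.
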(event EventBeginPlay)

(event Collision|EventActorBeginOverlap
  (params (OtherActor :type Actor%20Object%20Reference)))

(event EventTick
  (params (DeltaSeconds :type Float%20%28single-precision%29)))

(event EventOnInteracted
  (params (Interacting%20Character :type BP%20Character%20Base%20Object%20Reference))
  (if (> (Utilities|Array|Length (Variables|Parameter|GetInteract%20Messages)) 1)
    (Default|DisplayMulti-PageDialogue Interacting%20Character (Variables|Parameter|GetInteract%20Messages))
    (else
      (Default|DisplayDialogue Interacting%20Character (Utilities|Array|Get(acopy) (Variables|Parameter|GetInteract%20Messages)) 0.0))))

(fn ConstructionScript
  (Utilities|Array|Add (Variables|/Game/MarkObjectSystem/Component/BP_MarkObjectsComponent.BP_MarkObjectsComponent_C|GetMeshes%20To%20Mark (Variables|Default|GetBP_MarkObjectsComponent)) (Variables|Default|GetStaticMesh)))