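; BP_Cauldron is an interactable that gives the interacting character the enchantment currently in play on the player controller.
; It keeps one character enchanted at a time by clearing the previous one first.
; With no active enchantment, or a Ghost-enchanted character inside a wall, it shows a message through the GameState's widget instead.
; TestEnchantment can override the active enchantment at BeginPlay, and the construction script registers the mesh with BPMarkObjectsComponent.
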(event EventBeginPlay
  (Utilities|FlowControl|Sequence
    (:then_0
      (bind _asbp_nolbplayer_controller (Utilities|Casting|CastToBP_NOLBPlayerController (Game|GetPlayerController 0)))
      (Variables|Internal|SetPlayer%20Controller _asbp_nolbplayer_controller)
      (if (Utilities|Enum|NotEqual(Enum) (Variables|Default|GetTest%20Enchantment) "NewEnumerator0")
        (Variables|/Game/Blueprints/GameMode/BP_NOLBPlayerController.BP_NOLBPlayerController_C|SetEnchantment%20In%20Play (Variables|Internal|GetPlayer%20Controller) (Variables|Default|GetTest%20Enchantment))))
    (:then_1
      (bind _asbp_no_one_left_behind_game_state (Utilities|Casting|CastToBP_NoOneLeftBehindGameState (Game|GetGameState)))
      (Variables|Internal|SetGame%20State _asbp_no_one_left_behind_game_state))))

(event EventOnInteracted
  (params (Interacting%20Character :type BP%20Character%20Base%20Object%20Reference))
  (if (Utilities|Enum|NotEqual(Enum) (Variables|/Game/Blueprints/GameMode/BP_NOLBPlayerController.BP_NOLBPlayerController_C|GetEnchantment%20In%20Play (Variables|Internal|GetPlayer%20Controller)) "NewEnumerator0")
    (if (not (Variables|/Game/Blueprints/GameMode/BP_NOLBPlayerController.BP_NOLBPlayerController_C|GetCharacter%20In%20Wall (Variables|Internal|GetPlayer%20Controller)))
      (Utilities|FlowControl|Sequence
        (:then_0
          ;[1 1 1] Disenchant an already enchanted character, if one exists
          (Utilities|IsValid (Variables|/Game/Blueprints/GameMode/BP_NOLBPlayerController.BP_NOLBPlayerController_C|GetEnchanted%20Character (Variables|Internal|GetPlayer%20Controller))
            (:Is%20Valid
              (Default|SetCharacterEnchantment (Variables|/Game/Blueprints/GameMode/BP_NOLBPlayerController.BP_NOLBPlayerController_C|GetEnchanted%20Character (Variables|Internal|GetPlayer%20Controller)) "NewEnumerator0"))))
        (:then_1
          (Default|SetCharacterEnchantment Interacting%20Character (Variables|/Game/Blueprints/GameMode/BP_NOLBPlayerController.BP_NOLBPlayerController_C|GetEnchantment%20In%20Play (Variables|Internal|GetPlayer%20Controller)))
          (Variables|/Game/Blueprints/GameMode/BP_NOLBPlayerController.BP_NOLBPlayerController_C|SetEnchanted%20Character (Variables|Internal|GetPlayer%20Controller) Interacting%20Character)))
      (else
        (Default|DisplayMessage (Variables|/Game/Blueprints/GameMode/BP_NoOneLeftBehindGameState.BP_NoOneLeftBehindGameState_C|GetMessage%20Widget (Variables|Internal|GetGame%20State)) "Someone with the Ghost Enchantment is in a wall! Move them first!" 4.0)))
    (else
      (Default|DisplayMessage (Variables|/Game/Blueprints/GameMode/BP_NoOneLeftBehindGameState.BP_NoOneLeftBehindGameState_C|GetMessage%20Widget (Variables|Internal|GetGame%20State)) "There's nothing in here! Find some ingredients and activate an enchantment!" 4.0))))

(fn ConstructionScript
  (Utilities|Array|Add (Variables|/Game/MarkObjectSystem/Component/BP_MarkObjectsComponent.BP_MarkObjectsComponent_C|GetMeshes%20To%20Mark (Variables|Default|GetBP_MarkObjectsComponent)) (Variables|Default|GetStaticMesh)))