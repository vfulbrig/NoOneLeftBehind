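; BP_Ingredient is a collectable ingredient that feeds the player's enchantment menu when collected.
; On BeginPlay it runs the parent logic, then binds AddIngredient to the inherited OnCollectedDispatch.
; AddIngredient passes its IngredientType to the EnchantmentMenuWidget on the collector's PlayerController.
; The overlap and Tick events are disabled, and the construction script only calls its parent.
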(event Custom|Add%20Ingredient
  (params (Collector :type BP%20Character%20Base%20Object%20Reference))
  (Default|UpdatewithIngredient (Variables|/Game/Blueprints/GameMode/BP_NOLBPlayerController.BP_NOLBPlayerController_C|GetEnchantment%20Menu%20Widget (Variables|/Game/Blueprints/Characters/BP_CharacterBase.BP_CharacterBase_C|GetPlayer%20Controller Collector)) (Variables|Default|GetIngredient%20Type)))

(event EventBeginPlay
  (|CallParentFunction)
  (EventDispatchers|AssignOnCollectedDispatch (delegate Custom|Add%20Ingredient)))

(event Collision|EventActorBeginOverlap
  (params (OtherActor :type Actor%20Object%20Reference))
  (|CallParentFunction OtherActor) ; This node is disabled and will not be called.\nDrag off pins to build functionality.
)

(event EventTick
  (params (DeltaSeconds :type Float%20%28single-precision%29))
  (|CallParentFunction DeltaSeconds) ; This node is disabled and will not be called.\nDrag off pins to build functionality.
)

(fn ConstructionScript
  (|CallParentFunction))