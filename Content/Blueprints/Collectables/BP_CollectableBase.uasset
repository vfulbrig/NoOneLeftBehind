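; Base Blueprint for collectable pickups that spin, bounce and are collected when a character overlaps them.
; Tick adds yaw at SpinSpeed, while a timeline scaled by BounceTime lerps the actor between its start location and BounceHeight above it, skipped at zero height.
; Overlap by a BP_CharacterBase fires the collected dispatcher with that collector, then destroys the actor.
; The dispatcher is bound to an empty OnCollected event.
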(event Custom|On%20Collected
  (params (Collector :type BP%20Character%20Base%20Object%20Reference)))

(event EventBeginPlay
  (Utilities|FlowControl|Sequence
    (:then_0
      (bind _output_get (Variables|Internal|SetOriginal%20Location (Transformation|GetActorLocation)))
      (Variables|Internal|SetBounce%20Apex (Math|Vector|MakeVector (.x _output_get) (.y _output_get) (+ (.z _output_get) (Variables|Animation|GetBounce%20Height))))
      (if (!= (Variables|Animation|GetBounce%20Height) 0.0)
        (Components|Timeline|SetPlayRate (Variables|Default|GetTL_BounceAnim) (/ 1.0 (Variables|Animation|GetBounce%20Time)))
        (bind _bounce_alpha (Timeline|TL_BounceAnim Play)
          (:Update
            (Transformation|SetActorLocation (Math|Vector|Lerp(Vector) (Variables|Internal|GetOriginal%20Location) (Variables|Internal|GetBounce%20Apex) _bounce_alpha) false false)))))
    (:then_1
      (EventDispatchers|BindEventtoOnCollectedDispatch (delegate Custom|On%20Collected)))))

(event Collision|EventActorBeginOverlap
  (params (OtherActor :type Actor%20Object%20Reference))
  ;[1 1 1] Begin Overlap
  (bind _asbp_character_base (Utilities|Casting|CastToBP_CharacterBase OtherActor))
  (Default|CallOnCollectedDispatch _asbp_character_base)
  (Actor|DestroyActor))

(event EventTick
  (params (DeltaSeconds :type Float%20%28single-precision%29))
  (bind _returnvalue (Transformation|GetActorRotation))
  ;[1 1 1] Tick
  (Transformation|SetActorRotation (Math|Rotator|MakeRotator (.roll _returnvalue) (.pitch _returnvalue) (+ (.yaw _returnvalue) (* (Variables|Animation|GetSpin%20Speed) DeltaSeconds)))))

(fn ConstructionScript)