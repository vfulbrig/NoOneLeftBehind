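; Game state for No One Left Behind that tracks the characters in play and lets player 0 swap possession between them.
; SwapCharacter cycles an index forward or back with wraparound, then possesses that character.
; Removing a possessed character swaps to the next first; RemoveCharacters queues everyone outside a keep list, and CleanRemovedCharacters later destroys them.
; BeginPlay also creates the on-screen character message widget.
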(event Custom|Swap%20Character
  (params (Prev? :type Boolean))
  (if (> (CallFunction|GetNumCharactersinPlay) 1)
    (Utilities|FlowControl|Sequence
      (:then_0
        ;[1 1 1] Set the current index to that of the character to be swapped to.
        (if Prev?
          (bind _result (Math|Integer|DecrementInt (Variables|Default|GetCurrent%20Character%20Index))
            (:%20%20
              (if (< _result 0)
                (Variables|Default|SetCurrent%20Character%20Index (Utilities|Array|LastIndex (Variables|Default|GetCharacters%20In%20Play))))))
          (else
            (bind _result_2 (Math|Integer|IncrementInt (Variables|Default|GetCurrent%20Character%20Index))
              (:%20%20
                (if (> _result_2 (Utilities|Array|LastIndex (Variables|Default|GetCharacters%20In%20Play)))
                  (Variables|Default|SetCurrent%20Character%20Index 0)))))))
      (:then_1
        ;[1 1 1] Swap to the character
        (Pawn|Possess (Game|GetPlayerController 0) (Utilities|Array|Get(acopy) (Variables|Default|GetCharacters%20In%20Play) (Variables|Default|GetCurrent%20Character%20Index)))))))

(event EventBeginPlay
  (bind _returnvalue (UserInterface|CreateWidget "/Game/Blueprints/UI/WBP_CharacterMessage.WBP_CharacterMessage_C" (Game|GetPlayerController 0)))
  (bind _output_get (Variables|Default|SetMessage%20Widget _returnvalue))
  (UserInterface|Viewport|AddtoViewport _output_get 0))

(fn ConstructionScript)

(fn AddCharacter
  (params (Character :type BP%20Character%20Base%20Object%20Reference))
  (Utilities|Array|Add (Variables|Default|GetCharacters%20In%20Play) Character))

(fn RemoveCharacter
  (params (Character :type BP%20Character%20Base%20Object%20Reference))
  (if (Default|GetIsPossessed Character)
    (CallFunction|SwapCharacter false))
  (Utilities|Array|RemoveItem (Variables|Default|GetCharacters%20In%20Play) Character))

(fn GetNumCharactersinPlay
  (return (Utilities|Array|Length (Variables|Default|GetCharacters%20In%20Play))))

(fn CleanRemovedCharacters
  (bind _removed_characters (Variables|Default|GetRemoved%20Characters))
  (while (> (Utilities|Array|Length (Variables|Default|GetRemoved%20Characters)) 0)
    (Actor|DestroyActor (Utilities|Array|Get(acopy) _removed_characters))
    (Utilities|Array|RemoveIndex _removed_characters)))

(fn RemoveCharacters
  (params (Character's%20To%20Keep :type Array%20of%20BP%20Character%20Base%20Object%20References))
  (bind _characters_in_play (Variables|Default|GetCharacters%20In%20Play))
  (bind _current_index (LocalVariables|GetCurrent%20Index))
  (bind _output (Utilities|Array|Get(acopy) _characters_in_play _current_index))
  (while (<= (LocalVariables|GetCurrent%20Index) (Utilities|Array|LastIndex (Variables|Default|GetCharacters%20In%20Play)))
    (if (Utilities|Array|ContainsItem Character's%20To%20Keep _output)
      (Math|Integer|IncrementInt (LocalVariables|GetCurrent%20Index))
      (else
        (Utilities|Array|Add (Variables|Default|GetRemoved%20Characters) _output)
        (CallFunction|RemoveCharacter _output)))))