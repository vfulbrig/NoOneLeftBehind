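; Player controller that owns the enchantment recipe menu and resets the enchantment system.
; On BeginPlay it creates the menu widget, feeds it the ingredient types found on placed BP_Ingredient actors, and clears any character's active enchantment.
; Input actions toggle the menu and forward scrolling and selection to the widget while it is open.
; Opening the menu shows the cursor, pauses the game and disables pawn input; closing reverses this.
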(event EventBeginPlay
  ;[1 1 1] Begin Blay
  (Class|WidgetBlueprintLibrary|SetFocustoGameViewport) ; Why do I have to tell UE to do this?
  ;;[1 1 1] Create the Enchantment Recipe widget.
  (bind _returnvalue (UserInterface|CreateWidget "/Game/Blueprints/UI/WBP_EnchantmentRecipeMenu.WBP_EnchantmentRecipeMenu_C" self))
  (bind _output_get (Variables|Magic|SetEnchantment%20Menu%20Widget _returnvalue))
  (UserInterface|Viewport|AddtoViewport _output_get 0)
  (CallFunction|ResetEnchantmentSystem))

(event Input|ActionEvents|InputActionEnchantmentMenu
  (params (Key :type Key%20Structure))
  ;[1 1 1] Toggling the Enchantment Menu
  (:Pressed
    (CallFunction|SetEnchantmentMenuOpen (not (Variables|Default|GetEnchantment%20Menu%20Open?)))))

(event Input|ActionEvents|InputActionMenuUp
  (params (Key :type Key%20Structure))
  ;[1 1 1] Menu Scrolling
  (:Pressed
    (if (Variables|Default|GetEnchantment%20Menu%20Open?)
      (Default|ScrollRecipeSelection (Variables|Magic|GetEnchantment%20Menu%20Widget) false))))

(event Input|ActionEvents|InputActionMenuDown
  (params (Key :type Key%20Structure))
  ;[1 1 1] Menu Scrolling
  (:Pressed
    (if (Variables|Default|GetEnchantment%20Menu%20Open?)
      (Default|ScrollRecipeSelection (Variables|Magic|GetEnchantment%20Menu%20Widget) true))))

(event Input|ActionEvents|InputActionMenuExit
  (params (Key :type Key%20Structure))
  ;[1 1 1] Exit Enchantment Menu
  (:Pressed
    (CallFunction|SetEnchantmentMenuOpen false)))

(event Input|ActionEvents|InputActionMenuSelect
  (params (Key :type Key%20Structure))
  ;[1 1 1] Menu Select
  (:Pressed
    (if (Variables|Default|GetEnchantment%20Menu%20Open?)
      (Default|TryActivateSelectedWidget (Variables|Magic|GetEnchantment%20Menu%20Widget)))))

(fn ConstructionScript)

(fn ResetEnchantmentSystem
  (Utilities|FlowControl|Sequence
    (:then_0
      ;[1 1 1] UI Reset
      (bind _outactors (Actor|GetAllActorsOfClass "/Game/Blueprints/Collectables/BP_Ingredient.BP_Ingredient_C"))
      (for _array_element _outactors
        (Utilities|Array|Add (LocalVariables|GetIngredients%20In%20Play) (Variables|/Game/Blueprints/Collectables/BP_Ingredient.BP_Ingredient_C|GetIngredient%20Type _array_element)))
      (Default|PrepareEnchantmentUI (Variables|Magic|GetEnchantment%20Menu%20Widget) (LocalVariables|GetIngredients%20In%20Play)))
    (:then_1
      (Variables|Magic|SetEnchantment%20In%20Play "NewEnumerator0")
      (Utilities|IsValid (Variables|Magic|GetEnchanted%20Character)
        (:Is%20Valid
          (Default|SetCharacterEnchantment (Variables|Magic|GetEnchanted%20Character) "NewEnumerator0")
          (Variables|Magic|SetEnchanted%20Character 0))))))

(fn SetEnchantmentMenuOpen
  (params (Enchantment%20Menu%20Open :type Boolean))
  (bind _returnvalue (Pawn|GetControlledPawn))
  (Variables|Default|SetEnchantment%20Menu%20Open? Enchantment%20Menu%20Open)
  (Widget|SetVisibility (Variables|Magic|GetEnchantment%20Menu%20Widget) (select (Variables|Default|GetEnchantment%20Menu%20Open?) "SelfHitTestInvisible" "Collapsed"))
  (Variables|Default|SetbShowMouseCursor (Variables|Default|GetEnchantment%20Menu%20Open?))
  (Game|SetGamePaused (Variables|Default|GetEnchantment%20Menu%20Open?))
  (if (Variables|Default|GetEnchantment%20Menu%20Open?)
    (Input|DisableInput _returnvalue 0)
    (Default|ResetSelection (Variables|Magic|GetEnchantment%20Menu%20Widget))
    (Default|ClearFeedbackText (Variables|Magic|GetEnchantment%20Menu%20Widget))
    (else
      (Input|EnableInput _returnvalue 0))))