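; Actor component that marks and unmarks objects with an outline by toggling custom depth rendering on their meshes.
; MarkObject enables custom depth with a given stencil value, and UnmarkObejct disables it and resets the stencil to zero.
; Both branch on mesh type: static meshes come from the MeshesToMark array, while skeletal unmarking looks up the owner's skeletal mesh component.
; Invalid meshes print an error.
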(event Custom|MarkObject
  (params (MeshType :type E_MeshType%20Enum :default "NewEnumerator0") (Stencil%20Value :type Integer))
  (switch Utilities|FlowControl|Switch|SwitchonE_MeshType MeshType
    (:NewEnumerator0
      (for _array_element (Variables|Default|GetMeshes%20To%20Mark)
        ;[0 0 0] Turn On Outline for Static Mesh
        (Utilities|IsValid _array_element
          (:Is%20Valid
            (Rendering|SetRenderCustomDepth _array_element true)
            (Rendering|SetCustomDepthStencilValue _array_element Stencil%20Value))
          (:Is%20Not%20Valid
            (Development|PrintString "ERROR: Static Mesh Is Invalid!" true true "(R=1.000000,G=0.000000,B=0.000000,A=1.000000)")))))
    (:NewEnumerator1
      ;[0 0 0] Turn On Outline for Skeletal Mesh
      (Utilities|IsValid _array_element
        (:Is%20Valid
          (Rendering|SetRenderCustomDepth _array_element true)
          (Rendering|SetCustomDepthStencilValue _array_element Stencil%20Value))
        (:Is%20Not%20Valid
          (Development|PrintString "ERROR: Skeletal Mesh Is Invalid!" true true "(R=1.000000,G=0.000000,B=0.000000,A=1.000000)"))))))

(event Custom|UnmarkObejct
  (bind _returnvalue (Components|GetOwner))
  (bind _returnvalue_2 (Actor|GetComponentbyClass _returnvalue "/Script/Engine.SkeletalMeshComponent"))
  (switch Utilities|FlowControl|Switch|SwitchonE_MeshType (stale Custom|MarkObject MeshType)
    (:NewEnumerator0
      (for _array_element (Variables|Default|GetMeshes%20To%20Mark)
        ;[0 0 0] Turn Off Outline for Static Mesh
        (Utilities|IsValid _array_element
          (:Is%20Valid
            (Rendering|SetRenderCustomDepth _array_element false)
            (Rendering|SetCustomDepthStencilValue _array_element 0))
          (:Is%20Not%20Valid
            (Development|PrintString "ERROR: Static Mesh Is Invalid!" true true "(R=1.000000,G=0.000000,B=0.000000,A=1.000000)")))))
    (:NewEnumerator1
      ;[0 0 0] Turn Off Outline for Skeletal Mesh
      (Utilities|IsValid _returnvalue_2
        (:Is%20Valid
          (Rendering|SetRenderCustomDepth _returnvalue_2 false)
          (Rendering|SetCustomDepthStencilValue _returnvalue_2 0))
        (:Is%20Not%20Valid
          (Development|PrintString "ERROR: Skeletal Mesh Is Invalid!" true true "(R=1.000000,G=0.000000,B=0.000000,A=1.000000)"))))))