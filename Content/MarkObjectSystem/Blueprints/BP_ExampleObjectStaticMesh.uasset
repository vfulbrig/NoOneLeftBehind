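; Example static mesh actor for the mark object system that highlights itself and shows the player's distance to it.
; On player interaction, or at BeginPlay if flagged, it marks its mesh through BPMarkObjectsComponent with a stencil value and attaches a screen-space distance widget.
; A looping timer updates the distance and lerps the text height by range.
; The mark and widget clear after an optional duration or when the player overlaps the sphere.
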(event OnComponentBeginOverlap(Sphere)
  (params (OverlappedComponent :type Primitive%20Component%20Object%20Reference) (OtherActor :type Actor%20Object%20Reference) (OtherComp :type Primitive%20Component%20Object%20Reference) (OtherBodyIndex :type Integer) (bFromSweep :type Boolean) (SweepResult :type Hit%20Result%20Structure%20%28by%20ref%29))
  ;[1 0 0] If you don't want to unmark object automatically when you overlap sphere just unplug this event or delete code and sphere colission.
  ;;[0 0 0] Remove Mark after overlapping sphere
  (if (== OtherActor (Game|GetPlayerCharacter 0))
    (if (Variables|Private|GetMarkedActive)
      (Default|UnmarkObejct (Variables|Default|GetBP_MarkObjectsComponent))
      (CallFunction|RemoveDistanceText))))

(event Custom|AddDistanceText
  ;[0 0 0] Distance Text Widget
  (Variables|Default|GetDistanceWidgetComponent
    (:then)
    (:else
      (Utilities|FlowControl|Sequence
        (:then_0
          (CallFunction|CreateandAttachDistanceTextWidget (Variables|Default|GetStaticMesh)))
        (:then_1
          (|GetDistanceToMarkedObjectAndSetTextLocationNode))))))

(event Custom|RemoveDistanceText
  ;[0 0 0] Distance Text Widget
  (bind _distancewidgetcomponent (Variables|Default|GetDistanceWidgetComponent)
    (:then
      (Components|DestroyComponent _distancewidgetcomponent)
      (Utilities|Time|ClearandInvalidateTimerbyHandle (Variables|Private|GetGetDistanceToMarkedObjectTimer)))
    (:else)))

(event EventStartInteraction
  (bind _bp_markobjectscomponent (Variables|Default|GetBP_MarkObjectsComponent))
  ;[0 0 0] Player Interaction
  (if (Variables|MOS|GetCanBeTriggeredByPlayer?)
    ;[0 0 0] BeginPlay
    (Default|MarkObject _bp_markobjectscomponent "NewEnumerator0" 1)
    (CallFunction|AddDistanceText)
    (Variables|Private|SetMarkedActive true)
    (if (Variables|MOS|GetTemporaryMark)
      (Utilities|FlowControl|Delay (Variables|MOS|GetTemporaryMarkDuration))
      (Default|UnmarkObejct _bp_markobjectscomponent)
      (CallFunction|RemoveDistanceText))))

(event EventBeginPlay
  (bind _bp_markobjectscomponent (Variables|Default|GetBP_MarkObjectsComponent))
  ;[0 0 0] BeginPlay
  (if (Variables|MOS|GetMarkedOnStart)
    (Default|MarkObject _bp_markobjectscomponent "NewEnumerator0" 1)
    (CallFunction|AddDistanceText)
    (Variables|Private|SetMarkedActive true)
    (if (Variables|MOS|GetTemporaryMark)
      (Utilities|FlowControl|Delay (Variables|MOS|GetTemporaryMarkDuration))
      (Default|UnmarkObejct _bp_markobjectscomponent)
      (CallFunction|RemoveDistanceText))))

(fn ConstructionScript)

(fn CreateandAttachDistanceTextWidget
  (params (Target :type Scene%20Component%20Object%20Reference))
  (bind _returnvalue (UserInterface|CreateWidget "/Game/MarkObjectSystem/Widgets/DistanceCounter/WBP_DistanceCounter.WBP_DistanceCounter_C" (Game|GetPlayerController 0)))
  (bind _output_get (Variables|Widget|SetWB_DistanceWidget _returnvalue))
  (bind _returnvalue_2 (AddComponent|AddWidgetComponent false))
  (bind _output_get_2 (Variables|Default|SetDistanceWidgetComponent _returnvalue_2))
  (UserInterface|SetWidget _output_get_2 _output_get)
  (Class|WidgetComponent|SetWidgetSpace _output_get_2 "Screen")
  (Class|WidgetComponent|SetDrawatDesiredSize _output_get_2 true)
  (Collision|SetCollisionEnabled _output_get_2 "NoCollision")
  (Transformation|AttachComponentToComponent _output_get_2 Target "None" "SnapToTarget" "SnapToTarget" "SnapToTarget" true))

(event Custom|GetDistanceToMarkedObject
  (bind _returnvalue (Transformation|GetActorLocation))
  (bind _returnvalue_2 (Game|GetPlayerCharacter 0))
  (bind _returnvalue_3 (Transformation|GetActorLocation _returnvalue_2))
  (bind _returnvalue_4 (- _returnvalue_3 _returnvalue))
  (bind _returnvalue_5 (Math|Vector|VectorLength _returnvalue_4))
  (Default|UpdateDistance (Variables|Widget|GetWB_DistanceWidget) (Math|Float|Truncate (select (<= _returnvalue_5 0.0) 0.0 _returnvalue_5)))
  (Transformation|SetRelativeLocation (Variables|Default|GetDistanceWidgetComponent) (Math|Vector|Lerp(Vector) (Math|Vector|MakeVector 0.0 0.0 (Variables|MOS|GetCloseRangeTextHeight)) (Math|Vector|MakeVector 0.0 0.0 (Variables|MOS|GetLongRangeTextHeight)) (Math|Float|Clamp(Float) (/ _returnvalue_5 2.5e+03))) false false))